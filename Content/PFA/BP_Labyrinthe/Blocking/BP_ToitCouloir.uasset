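; Labyrinth blocking piece, named as a corridor roof, that randomizes its static mesh for visual variety.
; The construction script assigns a random mesh from the LeMeshUltime array, then adds a 90-degree world yaw with a one-in-four chance.
; The random picks are unseeded, so the look can change whenever construction reruns.
; The event graph holds only disabled placeholder events, so it adds no runtime logic.
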(event EventBeginPlay)

(event Collision|EventActorBeginOverlap
  (params (OtherActor :type Actor%20Object%20Reference)))

(event EventTick
  (params (DeltaSeconds :type Float%20%28single-precision%29)))

(fn ConstructionScript
  (bind _staticmesh (Variables|Default|GetStaticMesh))
  (bind _returnvalue (Transformation|GetWorldRotation _staticmesh))
  (Components|StaticMesh|SetStaticMesh (Variables|Default|GetStaticMesh) (.OutItem (Utilities|Array|Random (Variables|Default|GetLeMeshUltime))))
  (if (== (Math|Random|RandomIntegerinRange 0 3) 1)
    (Transformation|SetWorldRotation _staticmesh (Math|Rotator|MakeRotator (.roll _returnvalue) (.pitch _returnvalue) (+ (.yaw _returnvalue) 9e+01)) false false)))