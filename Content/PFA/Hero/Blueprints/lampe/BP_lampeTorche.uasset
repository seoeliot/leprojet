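; BP_lampeTorche is the hero's flashlight actor, built around a SpotLight.
; Pressing the Lumiere input action toggles the SpotLight's visibility.
; Disconnected logic that never runs would smoothly follow the player camera, interpolating location toward a camera-relative offset and rotation toward the camera's rotation.
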(event Input|ActionEvents|InputActionLumiere
  (params (Key :type Key%20Structure :default "None"))
  (:Pressed
    (Rendering|ToggleVisibility (Variables|Default|GetSpotLight) false)))

(fn ConstructionScript)