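; Lever actor that temporarily moves its associated door when its activation event fires.
; It finds the first actor of the door class referenced through NewVar0, calls Move on it and tilts its own cube as the handle.
; After a short delay it reverses both changes.
; A DoOnce, reset at the end of the cycle, blocks retriggering while the lever is active.
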(event Custom|resetdoonce
  (bind _cube (Variables|Default|GetCube))
  (bind _returnvalue (Transformation|GetWorldRotation _cube))
  (Utilities|FlowControl|DoOnce false) ; enters at Reset
)

(event Custom|child1activatin
  (bind _cube (Variables|Default|GetCube))
  (bind _returnvalue (Transformation|GetWorldRotation _cube))
  (Utilities|FlowControl|DoOnce false
    (:Completed
      (bind _outactors (Actor|GetAllActorsOfClass (Utilities|Struct|Breakstruct_levierXporte (Variables|Default|GetNewVar_0))))
      (Default|Move (Utilities|Array|Get(acopy) _outactors) -3e+02)
      (Transformation|SetWorldRotation _cube (Math|Rotator|MakeRotator (+ (.roll _returnvalue) 3e+01) (.pitch _returnvalue) (.yaw _returnvalue)) false false)
      (Utilities|FlowControl|Delay 3.0)
      (Transformation|SetWorldRotation _cube (Math|Rotator|MakeRotator (+ (.roll _returnvalue) -3e+01) (.pitch _returnvalue) (.yaw _returnvalue)) false false)
      (Default|Move (Utilities|Array|Get(acopy) _outactors) 3e+02)
      (CallFunction|Resetdoonce))))

(event EventBeginPlay)

(event Collision|EventActorBeginOverlap
  (params (OtherActor :type Actor%20Object%20Reference)))

(event EventTick
  (params (DeltaSeconds :type Float%20%28single-precision%29)))

(fn ConstructionScript)