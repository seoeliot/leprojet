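; Big lever actor that starts the timed puzzle of room S1 or S2, as selected by its room struct.
; BeginPlay copies that room's maximum time from GI_Main into the struct.
; Activation runs through a DoOnce, tilts the lever down, then sets the room's activated flag in GI_Main and calls its AppelSalle function with the puzzle time.
; EnigmeFinis raises the lever and resets the DoOnce for another activation.
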(event Custom|resetdoonce
  (bind _levier (Variables|Default|GetLevier))
  (bind _struct (Variables|Default|GetStruct))
  (bind _returnvalue (Transformation|GetWorldRotation _levier))
  (Utilities|FlowControl|DoOnce false) ; enters at Reset
)

(event Custom|EnigmeFinis
  (bind _levier (Variables|Default|GetLevier))
  (bind _returnvalue (Transformation|GetWorldRotation _levier))
  ;[1 1 1] Levier qui remonte
  (Transformation|SetWorldRotation _levier (Math|Rotator|MakeRotator 0.0 (.pitch _returnvalue) (.yaw _returnvalue)) false false)
  (CallFunction|Resetdoonce))

(event Custom|ActivationGrandLevier
  (bind _levier (Variables|Default|GetLevier))
  (bind _struct (Variables|Default|GetStruct))
  (bind _returnvalue (Transformation|GetWorldRotation _levier))
  (Utilities|FlowControl|DoOnce false
    (:Completed
      ;[1 1 1] Levier qui descend
      (Transformation|SetWorldRotation _levier (Math|Rotator|MakeRotator -6e+01 (.pitch _returnvalue) (.yaw _returnvalue)) false false)
      (Development|PrintString "Début de l'énigme")
      (Utilities|FlowControl|Sequence
        (:then_0
          (Utilities|FlowControl|DoOnce false))
        (:then_1
          (switch string (.lasale _struct)
            (:S1
              (bind _asgi_main (Utilities|Casting|CastToGI_Main (Game|GetGameInstance)))
              ;[1 1 1] Enigme commence
              (Variables|/Game/PFA/GI_Main.GI_Main_C|SetS1_LevierActiver _asgi_main true)
              (Default|AppelSalle1 _asgi_main (.letempsdelénigme _struct)))
            (:S2
              (bind _asgi_main_2 (Utilities|Casting|CastToGI_Main (Game|GetGameInstance)))
              (Variables|/Game/PFA/GI_Main.GI_Main_C|SetS2_LevierActiver _asgi_main_2 true)
              (Default|AppelSalle2 _asgi_main_2 (.letempsdelénigme _struct)))))))))

(event EventBeginPlay
  ;[0 1 0.8833] Le temps
  (switch string (Utilities|Struct|Breakstruc_levierXsalle (Variables|Default|GetStruct))
    (:S1
      (bind _asgi_main (Utilities|Casting|CastToGI_Main (Game|GetGameInstance)))
      (Variables|Default|SetStruct (Utilities|Struct|Makestruc_levierXsalle (Utilities|Struct|Breakstruc_levierXsalle (Variables|Default|GetStruct)) (Variables|/Game/PFA/GI_Main.GI_Main_C|GetS1_tempsMax _asgi_main))))
    (:S2
      (bind _asgi_main_2 (Utilities|Casting|CastToGI_Main (Game|GetGameInstance)))
      (Variables|Default|SetStruct (Utilities|Struct|Makestruc_levierXsalle (Utilities|Struct|Breakstruc_levierXsalle (Variables|Default|GetStruct)) (Variables|/Game/PFA/GI_Main.GI_Main_C|GetS2_tempsMax _asgi_main_2))))))

(fn ConstructionScript)