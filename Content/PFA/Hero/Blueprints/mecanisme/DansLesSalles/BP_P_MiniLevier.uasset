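; Mini lever actor for room puzzles, each instance set up with a room (S1 or S2) and a letter.
; On activation, if GI_Main flags that room's levers as active, a DoOnce tilts the lever down and passes its letter to the room's add function in GI_Main.
; EnigmeFinis raises the lever back up and resets the DoOnce, which can also be reset on its own.
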(event Custom|resetdoonce
  (bind _struct (Variables|Default|GetStruct))
  (bind _levier (Variables|Default|GetLevier))
  (bind _returnvalue (Transformation|GetWorldRotation _levier))
  (Utilities|FlowControl|DoOnce false) ; enters at Reset
)

(event Custom|ActivationMiniLevier
  (bind _struct (Variables|Default|GetStruct))
  (bind _levier (Variables|Default|GetLevier))
  (bind _returnvalue (Transformation|GetWorldRotation _levier))
  ;[1 1 1] test enigme commence ?
  (switch string (Utilities|Struct|Breakstruct_levierXlettre (Variables|Default|GetStruct))
    (:S1
      (bind _asgi_main (Utilities|Casting|CastToGI_Main (Game|GetGameInstance)))
      (if (Variables|/Game/PFA/GI_Main.GI_Main_C|GetS1_LevierActiver _asgi_main)
        (Utilities|FlowControl|DoOnce false :!label _label
          (:Completed
            ;[1 1 1] Levier qui descend
            (Transformation|SetWorldRotation _levier (Math|Rotator|MakeRotator (.roll _returnvalue) -1.2e+02 (.yaw _returnvalue)) false false)
            (switch string (.lasalle _struct)
              (:S1
                ;[1 1 1] Les appel sur les salles
                (bind _asgi_main_2 (Utilities|Casting|CastToGI_Main (Game|GetGameInstance)))
                (Default|S1Ajout _asgi_main_2 (.lalettre _struct)))
              (:S2
                (bind _asgi_main_3 (Utilities|Casting|CastToGI_Main (Game|GetGameInstance)))
                (Default|S2Ajout _asgi_main_3 (.lalettre _struct))))))))
    (:S2
      (bind _asgi_main_4 (Utilities|Casting|CastToGI_Main (Game|GetGameInstance)))
      (if (Variables|/Game/PFA/GI_Main.GI_Main_C|GetS2_LevierActiver _asgi_main_4)
        (goto _label)))))

(event Custom|EnigmeFinis
  (bind _levier (Variables|Default|GetLevier))
  (bind _returnvalue (Transformation|GetWorldRotation _levier))
  ;[1 1 1] Levier qui remonte
  (Transformation|SetWorldRotation _levier (Math|Rotator|MakeRotator (.roll _returnvalue) 0.0 (.yaw _returnvalue)) false false)
  (CallFunction|Resetdoonce))

(fn ConstructionScript)