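; Timed pressure plate that opens an associated door when the first-person character steps on it while GI_Main's HaveFire is set; otherwise it prints a hint.
; Activation lowers the plate, moves the first door actor of the configured class and calls Compte on the game instance.
; After the delay, if CanPlaque2 is true, plate and door move back and the DoN gate resets for reuse.
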(event OnComponentBeginOverlap(boxcolision)
  (params (OverlappedComponent :type Primitive%20Component%20Object%20Reference) (OtherActor :type Actor%20Object%20Reference) (OtherComp :type Primitive%20Component%20Object%20Reference) (OtherBodyIndex :type Integer) (bFromSweep :type Boolean) (SweepResult :type Hit%20Result%20Structure%20%28by%20ref%29))
  (bind _infoplaque (Variables|Default|GetInfoPlaque))
  (bind _plaque (Variables|Default|Getplaque))
  (bind _nombredesec (Variables|Default|GetNombreDeSec))
  (Utilities|Casting|CastToFirstPersonCharacter OtherActor)
  (bind _asgi_main (Utilities|Casting|CastToGI_Main (Game|GetGameInstance)))
  (if (Variables|/Game/PFA/GI_Main.GI_Main_C|GetHaveFire _asgi_main)
    (Utilities|FlowControl|DoN 1
      (:Exit
        (Development|PrintString "Ouverture de la porte" true true "(R=0.000000,G=0.660000,B=1.000000,A=1.000000)" 3.0)
        (bind _outactors (Actor|GetAllActorsOfClass (Utilities|Struct|Breakstruct_plaqueXporte (Variables|Default|GetStruct_plaqueXporte))))
        ;[0.2225 1 0.1422] MOVE
        (Default|Move (Utilities|Array|Get(acopy) _outactors) -3.5e+02)
        (Transformation|SetWorldLocation _plaque (Math|Vector|MakeVector (.x (.location _infoplaque)) (.y (.location _infoplaque)) (+ (.z (.location _infoplaque)) -14.0)) false false)
        (bind _asgi_main_2 (Utilities|Casting|CastToGI_Main (Game|GetGameInstance)))
        (Variables|/Game/PFA/GI_Main.GI_Main_C|SetCanPlaque2?PositionHaute _asgi_main_2 true)
        (Default|Compte _asgi_main_2 _nombredesec)
        (Utilities|FlowControl|Delay _nombredesec)
        (if (Variables|/Game/PFA/GI_Main.GI_Main_C|GetCanPlaque2? _asgi_main_2)
          (Transformation|SetWorldLocation _plaque (Math|Vector|MakeVector (.x (.location _infoplaque)) (.y (.location _infoplaque)) (.z (.location _infoplaque))) false false)
          ;[0.2225 1 0.1422] MOVE
          (Default|Move (Utilities|Array|Get(acopy) _outactors) 3.5e+02)
          (CallFunction|OnPeutRelancer)
          (bind _asgi_main_3 (Utilities|Casting|CastToGI_Main (Game|GetGameInstance)))
          (Variables|/Game/PFA/GI_Main.GI_Main_C|SetCanPlaque2?PositionHaute _asgi_main_3 false))))
    (else
      (Development|PrintString "Je ne peux pas encore activer cette plaque, je dervais aller voir ailleurs" true true "(R=0.000000,G=0.660000,B=1.000000,A=1.000000)" 5.0))))

(event Custom|On%20peut%20relancer
  (bind _infoplaque (Variables|Default|GetInfoPlaque))
  (bind _plaque (Variables|Default|Getplaque))
  (bind _nombredesec (Variables|Default|GetNombreDeSec))
  (Utilities|FlowControl|DoN 1) ; enters at Reset
)

(event EventBeginPlay
  (Variables|Default|SetInfoPlaque (Transformation|GetWorldTransform (Variables|Default|Getplaque))))

(fn ConstructionScript)