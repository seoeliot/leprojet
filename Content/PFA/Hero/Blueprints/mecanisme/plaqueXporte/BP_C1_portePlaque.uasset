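; BP_C1_portePlaque is a trigger actor in the plate-and-door mechanism that stops door 1 from descending again, as its debug message indicates.
; When the FirstPersonCharacter enters the BoxEntrée volume, it reads CanPlaque1PositionHaute from the GI_Main game instance.
; If that flag is true, it clears CanPlaque1 on the game instance, prints the message and destroys itself, making it single-use.
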(event OnComponentBeginOverlap(BoxEntrée)
  (params (OverlappedComponent :type Primitive%20Component%20Object%20Reference) (OtherActor :type Actor%20Object%20Reference) (OtherComp :type Primitive%20Component%20Object%20Reference) (OtherBodyIndex :type Integer) (bFromSweep :type Boolean) (SweepResult :type Hit%20Result%20Structure%20%28by%20ref%29))
  (Utilities|Casting|CastToFirstPersonCharacter OtherActor)
  (bind _asgi_main (Utilities|Casting|CastToGI_Main (Game|GetGameInstance)))
  (if (Variables|/Game/PFA/GI_Main.GI_Main_C|GetCanPlaque1?PositionHaute _asgi_main)
    (Variables|/Game/PFA/GI_Main.GI_Main_C|SetCanPlaque1? _asgi_main false)
    (Development|PrintString "La porte ne descends plus")
    (Actor|DestroyActor)))

(event EventBeginPlay
  (|CallParentFunction) ; This node is disabled and will not be called.\nDrag off pins to build functionality.
)

(event Collision|EventActorBeginOverlap
  (params (OtherActor :type Actor%20Object%20Reference))
  (|CallParentFunction OtherActor) ; This node is disabled and will not be called.\nDrag off pins to build functionality.
)

(event EventTick
  (params (DeltaSeconds :type Float%20%28single-precision%29))
  (|CallParentFunction DeltaSeconds) ; This node is disabled and will not be called.\nDrag off pins to build functionality.
)

(fn ConstructionScript
  (|CallParentFunction))