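; Pressure plate actor that moves an associated door when something overlaps its collision box.
; On overlap it moves the first actor found of the PorteAssocié class and sinks the plate mesh, then restores both after a fixed delay.
; A DoN node blocks retriggering during the cycle until the OnPeutRelancer event resets it.
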(event OnComponentBeginOverlap(boxcolision)
  (params (OverlappedComponent :type Primitive%20Component%20Object%20Reference) (OtherActor :type Actor%20Object%20Reference) (OtherComp :type Primitive%20Component%20Object%20Reference) (OtherBodyIndex :type Integer) (bFromSweep :type Boolean) (SweepResult :type Hit%20Result%20Structure%20%28by%20ref%29))
  (bind _infoplaque (Variables|Default|GetInfoPlaque))
  (bind _plaque (Variables|Default|Getplaque))
  (Utilities|FlowControl|DoN 1
    (:Exit
      (bind _outactors (Actor|GetAllActorsOfClass (Utilities|Struct|Breakstruct_levierXporte (Variables|Default|GetNewVar_0))))
      (Default|Move (Utilities|Array|Get(acopy) _outactors) -3e+02)
      (Transformation|SetWorldLocation _plaque (Math|Vector|MakeVector (.x (.location _infoplaque)) (.y (.location _infoplaque)) (+ (.z (.location _infoplaque)) -14.0)) false false)
      (Utilities|FlowControl|Delay 5.0)
      (Transformation|SetWorldLocation _plaque (Math|Vector|MakeVector (.x (.location _infoplaque)) (.y (.location _infoplaque)) (.z (.location _infoplaque))) false false)
      (Default|Move (Utilities|Array|Get(acopy) _outactors) 3e+02)
      (CallFunction|OnPeutRelancer))))

(event Custom|On%20peut%20relancer
  (bind _infoplaque (Variables|Default|GetInfoPlaque))
  (bind _plaque (Variables|Default|Getplaque))
  (Utilities|FlowControl|DoN 1) ; enters at Reset
)

(event EventBeginPlay
  (Variables|Default|SetInfoPlaque (Transformation|GetWorldTransform (Variables|Default|Getplaque))))

(event Collision|EventActorBeginOverlap
  (params (OtherActor :type Actor%20Object%20Reference)))

(event EventTick
  (params (DeltaSeconds :type Float%20%28single-precision%29)))

(fn ConstructionScript)