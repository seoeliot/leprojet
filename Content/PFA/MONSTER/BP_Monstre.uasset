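; Monster AI that patrols, hunts the first-person player and opens the death map on box overlap.
; Patrols alternate between random points around itself and around the player.
; PawnSensing sight or loud, close noise triggers a chase, while other noises raise speed, with "close" measured from world origin via VectorLength(Location).
; Looping countdown timers, refreshed by detections, return it to patrol, and state flags set footstep cadence.
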(event OnComponentBeginOverlap(Box)
  (params (OverlappedComponent :type Primitive%20Component%20Object%20Reference) (OtherActor :type Actor%20Object%20Reference) (OtherComp :type Primitive%20Component%20Object%20Reference) (OtherBodyIndex :type Integer) (bFromSweep :type Boolean) (SweepResult :type Hit%20Result%20Structure%20%28by%20ref%29))
  ;[1 1 1] KILL
  (Utilities|Casting|CastToFirstPersonCharacter OtherActor)
  (Game|OpenLevel(byObjectReference) "/Game/PFA/UI_HUD/map_mort.map_mort"))

(event OnHearNoise(PawnSensing)
  (params (Instigator :type Pawn%20Object%20Reference) (Location :type Vector%20%28by%20ref%29 :default "0, 0, 0") (Volume :type Float%20%28single-precision%29))
  (bind _returnvalue (Math|Vector|VectorLength Location))
  ;[1 0 1] SON
  (if (== Instigator (Game|GetPlayerCharacter 0))
    (if (>= Volume 0.9)
      (if (<= _returnvalue 5e+03)
        ;[1 0 0] RUN
        (CallFunction|RUN :!label _label)
        (Variables|JeFaisQuoi|SetIsRuning true)
        ;[0 1 0.8833] CDO
        (CallFunction|CallDoOnce)
        (else
          ;[0.0239 1 0] Accelération
          (Variables|/Script/Engine.CharacterMovementComponent|SetMaxWalkSpeed (Variables|Character|GetCharacterMovement) 3.5e+02 :!label _label_2)
          ;[0 0.09533 1] SON
          (if (Variables|Son|GetCanTespasloin?)
            (Audio|PlaySoundatLocation "/Game/PFA/MONSTER/audio/evenement/SC_mtespasloin.SC_mtespasloin" (Transformation|GetActorLocation) "0, 0, 0" 1.0 1.0 0.0 0 0 0)
            (Variables|Son|SetCanTespasloin? false))
          (Variables|JeFaisQuoi|SetIsSprinting true)
          ;[0 1 0.8833] CDO
          (CallFunction|CallDoOnceFaster)))
      (elif (>= Volume 0.3)
        (if (<= _returnvalue 1e+03)
          (goto _label)
          (else
            (goto _label_2)))))))

(event OnSeePawn(PawnSensing)
  (params (Pawn :type Pawn%20Object%20Reference))
  ;[1 0 1] VUE
  (Utilities|Casting|CastToFirstPersonCharacter Pawn)
  ;[1 0 0] RUN
  (CallFunction|RUN)
  (Variables|JeFaisQuoi|SetIsRuning true)
  ;[0 1 0.8833] CDO
  (CallFunction|CallDoOnce))

(event Custom|RUN
  (Utilities|FlowControl|Sequence
    (:then_0
      ;[1 1 1] TEST
      (Utilities|FlowControl|DoOnce false
        (:Completed
          (Audio|PlaySoundatLocation "/Game/PFA/MONSTER/audio/evenement/SC_ambianceRun.SC_ambianceRun" (Transformation|GetActorLocation (Game|GetPlayerCharacter 0)) "0, 0, 0" 1.0 1.0 0.0 0 0 0))))
    (:then_1
      ;[0 0.09533 1] SON
      (if (Variables|Son|GetCanRuning?)
        (Audio|PlaySoundatLocation "/Game/PFA/MONSTER/audio/evenement/SC_mrun.SC_mrun" (Transformation|GetActorLocation) "0, 0, 0" 1.0 1.0 0.0 0 0 0)
        (Variables|Son|SetCanRuning? false))
      ;[1 0 0] RUN
      (Variables|/Script/Engine.CharacterMovementComponent|SetMaxWalkSpeed (Variables|Character|GetCharacterMovement) 5e+02)
      (AI|AIMoveTo self "0, 0, 0" (Game|GetPlayerCharacter 0) 5e+01 false
        (:OnSuccess
          _)
        (:OnFail
          _))
      (CallFunction|RUN))
    (:then_2
      (Utilities|FlowControl|Delay 3e+01)
      (Class|GameplayStatics|ClearSoundMixModifiers))))

(event Custom|resettimerFaster
  ;[0 1 0.8833] CDO
  (Utilities|FlowControl|DoOnce false) ; enters at Reset
)

(event Custom|CallDoOnceFaster
  ;[0 1 0.8833] CDO
  (Utilities|FlowControl|DoOnce false
    (:Completed
      (CallFunction|Timer/faster))))

(event Custom|timer/vue
  ;[0 1 0.8833] TIMER/VUE
  (bind _returnvalue (Utilities|Time|SetTimerbyEvent (delegate Custom|compteur+1) 1.0 true))
  (Variables|compte|SetTimerRef _returnvalue))

(event Custom|compteur+1
  ;[0 1 0.8833] TIMER/VUE
  (if (< (Variables|compte|Getcompteur) 12)
    (if (Variables|JeFaisQuoi|GetIsRuning)
      (Variables|compte|Setcompteur 0))
    (Variables|compte|Setcompteur (+ 1 (Variables|compte|Getcompteur)))
    (Variables|JeFaisQuoi|SetIsRuning false)
    (else
      (Utilities|Time|ClearandInvalidateTimerbyHandle (Variables|compte|GetTimerRef))
      (Components|Movement|StopMovementImmediately (Variables|Character|GetCharacterMovement))
      (Variables|compte|Setcompteur 0)
      ;[0 0.09533 1] SON
      (Audio|PlaySoundatLocation "/Game/PFA/MONSTER/audio/evenement/SC_mjetairate.SC_mjetairate" (Transformation|GetActorLocation) "0, 0, 0" 1.0 1.0 0.0 0 0 0)
      (CallFunction|Resttimer)
      (CallFunction|ControlleDePatrouille)
      (Variables|Son|SetCanRuning? true))))

(event Custom|PatrouileJoueur
  ;[0.901 0.4068 0.006969] PatrouileJoueur
  (Variables|JeFaisQuoi|SetIsAlea? false)
  (Variables|/Script/Engine.CharacterMovementComponent|SetMaxWalkSpeed (Variables|Character|GetCharacterMovement) 3e+02)
  (AI|AIMoveTo self (.RandomLocation (AI|Navigation|GetRandomReachablePointinRadius (Transformation|GetActorLocation (Game|GetPlayerCharacter 0)) 3e+03 0 0)) 0 5.0 false
    (:OnSuccess
      _)
    (:OnFail
      _))
  (Utilities|FlowControl|Delay 2.0)
  (CallFunction|ControlleDePatrouille))

(event Custom|resttimer
  ;[0 1 0.8833] CDO
  (Utilities|FlowControl|DoOnce false) ; enters at Reset
)

(event Custom|CallDoOnce
  ;[0 1 0.8833] CDO
  (Utilities|FlowControl|DoOnce false
    (:Completed
      (CallFunction|Timer/vue))))

(event Custom|PatrouilleAlea
  ;[1 0.834 0.05432] PatrouileAlea
  (Variables|JeFaisQuoi|SetIsAlea? true)
  (Variables|/Script/Engine.CharacterMovementComponent|SetMaxWalkSpeed (Variables|Character|GetCharacterMovement) 2e+02)
  (AI|AIMoveTo self (.RandomLocation (AI|Navigation|GetRandomReachablePointinRadius (Transformation|GetActorLocation) 1e+04 0 0)) 0 5.0 false
    (:OnSuccess
      _)
    (:OnFail
      _))
  (Utilities|FlowControl|Delay 2.0)
  (CallFunction|ControlleDePatrouille))

(event Custom|PasDuMonstre
  (Utilities|Time|SetTimerbyEvent (delegate Custom|FaisDuBruit) 0.1 true))

(event Custom|timer/faster
  ;[0 1 0.8833] TIMER/FASTER
  (bind _returnvalue (Utilities|Time|SetTimerbyEvent (delegate Custom|copteur/faster+1) 1.0 true))
  (Variables|compte|SetTimerFasterRef _returnvalue))

(event Custom|copteur/faster+1
  ;[0 1 0.8833] TIMER/FASTER
  (if (< (Variables|compte|GetcompteurFaster) 15)
    (if (Variables|JeFaisQuoi|GetIsSprinting)
      (Variables|compte|SetcompteurFaster 0))
    (Variables|compte|SetcompteurFaster (+ 1 (Variables|compte|GetcompteurFaster)))
    (Variables|JeFaisQuoi|SetIsSprinting false)
    (else
      (Utilities|Time|ClearandInvalidateTimerbyHandle (Variables|compte|GetTimerFasterRef))
      (Components|Movement|StopMovementImmediately (Variables|Character|GetCharacterMovement))
      (Variables|compte|SetcompteurFaster 0)
      ;[0 0.09533 1] SON
      (Audio|PlaySoundatLocation "/Game/PFA/MONSTER/audio/evenement/SC_mjetairate.SC_mjetairate" (Transformation|GetActorLocation) "0, 0, 0" 1.0 1.0 0.0 0 0 0)
      (CallFunction|ResettimerFaster)
      (CallFunction|ControlleDePatrouille)
      (Variables|Son|SetCanTespasloin? true))))

(event Custom|FaisDuBruit
  (if (Variables|JeFaisQuoi|GetIsRuning)
    (Utilities|FlowControl|Delay 0.3)
    (Audio|PlaySoundatLocation "/Game/PFA/MONSTER/audio/pas/SC_pasm1.SC_pasm1" (Transformation|GetActorLocation) "0, 0, 0" 1.0 1.0 0.0 0 0 0)
    (Utilities|FlowControl|Delay 0.3)
    (Audio|PlaySoundatLocation "/Game/PFA/MONSTER/audio/pas/SC_pasm2.SC_pasm2" (Transformation|GetActorLocation) "0, 0, 0" 1.0 1.0 0.0 0 0 0)
    (elif (Variables|JeFaisQuoi|GetIsSprinting)
      (Utilities|FlowControl|Delay 1.0)
      (Audio|PlaySoundatLocation "/Game/PFA/MONSTER/audio/pas/SC_pasm1.SC_pasm1" (Transformation|GetActorLocation) "0, 0, 0" 1.0 1.0 0.0 0 0 0)
      (Utilities|FlowControl|Delay 1.0)
      (Audio|PlaySoundatLocation "/Game/PFA/MONSTER/audio/pas/SC_pasm2.SC_pasm2" (Transformation|GetActorLocation) "0, 0, 0" 1.0 1.0 0.0 0 0 0)
      (else
        (Utilities|FlowControl|Delay 2.0)
        (Audio|PlaySoundatLocation "/Game/PFA/MONSTER/audio/pas/SC_pasm1.SC_pasm1" (Transformation|GetActorLocation) "0, 0, 0" 1.0 1.0 0.0 0 0 0)
        (Utilities|FlowControl|Delay 2.0)
        (Audio|PlaySoundatLocation "/Game/PFA/MONSTER/audio/pas/SC_pasm2.SC_pasm2" (Transformation|GetActorLocation) "0, 0, 0" 1.0 1.0 0.0 0 0 0)))))

(event EventBeginPlay
  (Utilities|FlowControl|Delay 1.0)
  (CallFunction|PatrouileJoueur)
  (CallFunction|PasDuMonstre))

(fn ConstructionScript)

(fn ControlleDePatrouille
  (if (Variables|JeFaisQuoi|GetIsAlea?)
    (if (< (Variables|JeFaisQuoi|GetC_Alea) 3)
      (Variables|JeFaisQuoi|SetC_Alea (+ 1 (Variables|JeFaisQuoi|GetC_Alea)))
      (CallFunction|PatrouilleAlea)
      (else
        (Variables|JeFaisQuoi|SetC_Alea 0)
        (CallFunction|PatrouileJoueur)))
    (elif (< (Variables|JeFaisQuoi|GetC_Alea) 2)
      (Variables|JeFaisQuoi|SetC_Alea (+ 1 (Variables|JeFaisQuoi|GetC_Alea)))
      (CallFunction|PatrouileJoueur)
      (else
        (Variables|JeFaisQuoi|SetC_Alea 0)
        (CallFunction|PatrouilleAlea)))))